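; BP_Final_Level is a Blueprint that shows a timed series of on-screen notifications when play begins, apparently for the final level.
; BeginPlay creates widgets and adds each to the viewport, waiting MessageTime between them.
; The Text_Notification messages congratulate the player, then warn twice of an active gravity well.
; The second widget has no class or text set, and the last is not passed MessageTime.
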(event `self.ReceiveBeginPlay`
  (bind _message_time (`self.Message Time`))
  (bind _returnvalue (`|CreateWidget` "/Game/UMG/Text_Notification.Text_Notification_C" null "Congradulations on a job well done" _message_time))
  (`UserWidget.AddToViewport` _returnvalue 0)
  (`KismetSystemLibrary.Delay` _message_time)
  (bind _returnvalue_2 (`|CreateWidget` "/Game/UMG/Text_Notification.Text_Notification_C" null "" _message_time))
  (`UserWidget.AddToViewport` _returnvalue_2 0)
  (`KismetSystemLibrary.Delay` _message_time)
  (bind _returnvalue_3 (`|CreateWidget` "/Game/UMG/Text_Notification.Text_Notification_C" null "!!Caution Active Gravity Well!!" _message_time))
  (`UserWidget.AddToViewport` _returnvalue_3 0)
  (`KismetSystemLibrary.Delay` _message_time)
  (bind _returnvalue_4 (`|CreateWidget` "/Game/UMG/Text_Notification.Text_Notification_C" null "!!Caution Active Gravity Well!!"))
  (`UserWidget.AddToViewport` _returnvalue_4 0))

(fn `UserConstructionScript`)