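; BP_Orb is a physics-driven orb that drifts in random directions and can spawn the item type it carries.
; It applies a random impulse at start, and again on Tick whenever its summed axis speeds fall within the SpeedBumper limit.
; SpawnItem creates a BP_Item just above the sphere, gated by a DoOnce that AllowSpawning resets.
; Highlighting briefly shows the collisionless item mesh, using a retriggerable delay to hide it.
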(event `self.ReceiveBeginPlay`
  (bind _sm_sphere (`self.SM_Sphere`))
  (bind _item (`self.Item`))
  ;[1 1 1] Initalization
  (`PrimitiveComponent.SetMaterial` _sm_sphere 0 (`self.Orb_Color`))
  (`StaticMeshComponent.SetStaticMesh` _item (`self.Orb_Item_Type`))
  (`PrimitiveComponent.SetCollisionEnabled` _item "NoCollision")
  (`PrimitiveComponent.SetMaterial` _item 0 (`self.Orb_Item_Mat`))
  ;;[1 1 1] Todo: Figure out how to give the orb a random velocity at start
  (`PrimitiveComponent.AddImpulse` _sm_sphere (* (`KismetMathLibrary.RandomUnitVector`) (`self.Orb Speed`)) "None" false))

(event `/Game/Blueprints/Interactions.Spawn_Item`
  (bind (_returnvalue_x _returnvalue_y _returnvalue_z) (`KismetMathLibrary.BreakVector` (`SceneComponent.K2_GetComponentLocation` (`self.SM_Sphere`))))
  ;[1 1 1] Spawns Item
  (`/Engine/EditorBlueprintResources/StandardMacros.DoOnce` false :!label _label
    (:`Completed`
      (`|SpawnActorFromClass` "/Game/Blueprints/BP_Item.BP_Item_C" (`KismetMathLibrary.MakeTransform` (`KismetMathLibrary.MakeVector` _returnvalue_x _returnvalue_y (+ _returnvalue_z 10.0))) "Undefined" "OverrideRootScale" null (`self.Orb_Item_Type`) (`self.Orb_Item_Mat`) self null))))

(event `AllowSpawning`
  ;[1 1 1] Spawns Item
  (goto _label :!via `Reset`))

(event `self.ReceiveTick`
  (params (DeltaSeconds :type "Float (single-precision)"))
  (bind _sm_sphere (`self.SM_Sphere`))
  (bind (_returnvalue_x _returnvalue_y _returnvalue_z) (`KismetMathLibrary.BreakVector` (`SceneComponent.GetComponentVelocity` _sm_sphere)))
  ;[1 1 1] Death Stuff
  (if (`KismetMathLibrary.InRange_FloatFloat` (+ (`KismetMathLibrary.Abs` _returnvalue_x) (`KismetMathLibrary.Abs` _returnvalue_y) (`KismetMathLibrary.Abs` _returnvalue_z)) 0.0 (`self.Speed Bumper`))
    (`PrimitiveComponent.AddImpulse` _sm_sphere (* (`KismetMathLibrary.RandomUnitVector`) (`self.Orb Speed`)) "None" false)))

(event `Highlighting`
  (bind _item (`self.Item`))
  (`SceneComponent.SetVisibility` _item true false)
  (`KismetSystemLibrary.RetriggerableDelay` 0.5)
  (`SceneComponent.SetVisibility` _item false false))

(fn `UserConstructionScript`)