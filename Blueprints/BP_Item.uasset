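; BP_Item is a physics-driven item actor whose mesh and material come from its ItemType and ItemMat variables.
; BeginPlay applies both to ItemMesh and turns on physics simulation.
; Tick casts the player pawn to My_Pawn every frame and destroys the item once that pawn's Fups value drops to zero or below.
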(event `self.ReceiveBeginPlay`
  (bind _item_mesh (`self.Item Mesh`))
  ;[1 1 1] Initalization
  (`StaticMeshComponent.SetStaticMesh` _item_mesh (`self.Item_Type`))
  (`PrimitiveComponent.SetMaterial` _item_mesh 0 (`self.Item_Mat`))
  (`PrimitiveComponent.SetSimulatePhysics` _item_mesh true))

(event `self.ReceiveTick`
  (params (DeltaSeconds :type "Float (single-precision)"))
  ;[1 1 1] Death Stuff
  (if (<= (`/Game/Blueprints/My_Pawn.Fups` (cast `/Game/Blueprints/My_Pawn` (`GameplayStatics.GetPlayerPawn` 0) :!pure true)) 0)
    (`self.K2_DestroyActor`)))

(fn `UserConstructionScript`)